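; HUD for the multiplayer FPS that creates the player's UI widgets and draws a full-screen scope overlay.
; BeginPlay adds the container, a scoreboard for FFA, CTF and TDM, and the team/class select menu, hiding team buttons in Co Op and Single Player.
; Game mode comes from the GameInstance on the server, otherwise from the GameState.
; DrawHUD renders a dynamic scope material by ScopeOpacity; ShowCharacterStationMenu displays the pre-created station menu.
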(event Custom|ShowCharacterStationMenu
  (bind _returnvalue (Game|Player|GetOwningPlayerController))
  (UserInterface|Viewport|AddtoViewport (Variables|Default|GetCharacterStationMenuRef) 0)
  (Input|SetInputModeUIOnly _returnvalue (Variables|Default|GetCharacterStationMenuRef) "DoNotLock")
  (Variables|/Script/Engine.PlayerController|SetbShowMouseCursor _returnvalue true))

(event EventBeginPlay
  (bind _returnvalue (Game|Player|GetOwningPlayerController))
  (Utilities|FlowControl|Sequence
    (:then_0
      (bind _asgi_mp_fps (Utilities|Casting|CastToGI_MP_FPS (Game|GetGameInstance)))
      (Variables|Default|SetGameInstanceRef _asgi_mp_fps)
      (bind _asgs_mp_fps (Utilities|Casting|CastToGS_MP_FPS (Game|GetGameState)))
      (Variables|Default|SetGameStateRef _asgs_mp_fps))
    (:then_1
      (Networking|SwitchHasAuthority
        (:Authority
          (bind _returnvalue_2 (UserInterface|CreateWidget "/Game/MP_FPS/Widgets/Player/BPW_Container.BPW_Container_C" _returnvalue))
          (bind _output_get (Variables|Default|SetW_ContainerRef _returnvalue_2))
          (UserInterface|Viewport|AddtoViewport _output_get 0))))
    (:then_2
      (Networking|SwitchHasAuthority
        (:Authority
          (switch Utilities|FlowControl|Switch|SwitchonE_GameModes (select (Networking|IsServer) (Variables|/Game/MP_FPS/Blueprints/GI_MP_FPS.GI_MP_FPS_C|GetE_SelectedGameMode (Variables|Default|GetGameInstanceRef)) (Variables|/Game/MP_FPS/Blueprints/GS_MP_FPS.GS_MP_FPS_C|GetE_SelectedGameMode (Variables|Default|GetGameStateRef)))
            (:NewEnumerator1
              _)
            (:NewEnumerator2
              _)
            (:NewEnumerator3
              _))
          (bind _returnvalue_3 (UserInterface|CreateWidget "/Game/MP_FPS/Widgets/UI/BPW_ScoreBoard.BPW_ScoreBoard_C" _returnvalue))
          (bind _output_get_2 (Variables|Default|SetW_ScoreBoard _returnvalue_3))
          (UserInterface|Viewport|AddtoViewport _output_get_2 0))))
    (:then_3
      (Networking|SwitchHasAuthority
        (:Authority
          (bind _returnvalue_4 (UserInterface|CreateWidget "/Game/MP_FPS/Widgets/UI/BPW_TeamClassSelect.BPW_TeamClassSelect_C" _returnvalue))
          (bind _output_get_3 (Variables|Default|SetW_TeamSelect _returnvalue_4))
          (UserInterface|Viewport|AddtoViewport _output_get_3 0)
          (Input|SetInputModeUIOnly _returnvalue _output_get_3 "DoNotLock")
          (Variables|/Script/Engine.PlayerController|SetbShowMouseCursor _returnvalue true)
          (switch Utilities|FlowControl|Switch|SwitchonE_GameModes (select (Networking|IsServer) (Variables|/Game/MP_FPS/Blueprints/GI_MP_FPS.GI_MP_FPS_C|GetE_SelectedGameMode (Variables|Default|GetGameInstanceRef)) (Variables|/Game/MP_FPS/Blueprints/GS_MP_FPS.GS_MP_FPS_C|GetE_SelectedGameMode (Variables|Default|GetGameStateRef)))
            (:NewEnumerator4
              _)
            (:NewEnumerator0
              _))
          (Widget|SetVisibility (Variables|/Game/MP_FPS/Widgets/UI/BPW_TeamClassSelect.BPW_TeamClassSelect_C|Getteambuttons_vb (Variables|Default|GetW_TeamSelect)) "Hidden"))))
    (:then_4
      (bind _returnvalue_5 (Rendering|Material|CreateDynamicMaterialInstance "/Game/MP_FPS/Materials/M_Scope.M_Scope" :!class /Script/Engine.KismetMaterialLibrary))
      (Variables|Default|SetScopeMaterialRef _returnvalue_5))
    (:then_5
      (bind _returnvalue_6 (UserInterface|CreateWidget "/Game/MP_FPS/Widgets/UI/BPW_CharacterStation.BPW_CharacterStation_C" (Game|Player|GetOwningPlayerController)))
      (Variables|Default|SetCharacterStationMenuRef _returnvalue_6))))

(event EventDrawHUD
  (params (SizeX :type Integer) (SizeY :type Integer))
  (bind _scopematerialref (Variables|Default|GetScopeMaterialRef))
  (Utilities|IsValid _scopematerialref
    (:Is%20Valid
      (Rendering|Material|SetScalarParameterValue _scopematerialref "ScopeOpacity" (Variables|Default|GetScopeOpacity) :!class /Script/Engine.MaterialInstanceDynamic)
      (Canvas|DrawMaterial _scopematerialref 0.0 0.0 (Math|Conversions|ToFloat(Integer) SizeX) (Math|Conversions|ToFloat(Integer) SizeY) 0.0 0.0 1.0 1.0))))

(fn ConstructionScript)