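; BP_CoinSpawner_Master is a server-side spawner that scatters randomly typed coins over landscape inside a configurable box volume, capped at 25 in the level.
; A looping one-second timer on authority counts coins and sphere-traces from a random box point, with debug drawing.
; The trace end multiplies a second random point by a Z-only vector, zeroing X and Y.
; Landscape hits spawn BP_CoinMaster above the impact; other hits are skipped.
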(event Custom|SphereTrace
  (bind _spawnervolume (Variables|Default|GetSpawnerVolume))
  (bind _e_cointype (Variables|Default|GetE_CoinType))
  (bind _returnvalue (Transformation|GetWorldLocation _spawnervolume))
  (bind _returnvalue_2 (Components|Box|GetScaledBoxExtent _spawnervolume))
  (bind _returnvalue_3 (Math|Random|RandomPointinBoundingBox _returnvalue _returnvalue_2))
  (bind _outactors (Actor|GetAllActorsOfClass "/Game/MP_FPS/Blueprints/BP_CoinMaster.BP_CoinMaster_C"))
  (if (< (Utilities|Array|Length _outactors) 25)
    (Variables|Default|SetE_SelectedCoin (Utilities|Array|Get(acopy) _e_cointype (Math|Random|RandomIntegerinRange 0 (- (Utilities|Array|Length _e_cointype) 1))))
    (bind (_outhit _returnvalue_4) (Collision|SphereTraceByChannel _returnvalue_3 (* _returnvalue_3 "0, 0,-10000.000000") 1e+02 "TraceTypeQuery1" false (Utilities|Array|MakeArray self) "ForDuration"))
    (if _returnvalue_4
      (Utilities|Casting|CastToBP_CoinMaster (.HitActor (Collision|BreakHitResult _outhit))
        (:CastFailed
          (Utilities|Casting|CastToBP_Character_Master (.HitActor (Collision|BreakHitResult _outhit))
            (:CastFailed
              (Utilities|Casting|CastToLandscape (.HitActor (Collision|BreakHitResult _outhit)))
              (Game|SpawnActorfromClass "/Game/MP_FPS/Blueprints/BP_CoinMaster.BP_CoinMaster_C" (Math|Transform|MakeTransform (+ (.ImpactPoint (Collision|BreakHitResult _outhit)) "0, 0,100.000000") "0, 0, 0" "1,1,1") "AdjustIfPossibleButDontSpawnIfColliding" 0 (Variables|Default|GetE_SelectedCoin) 0))))))))

(event EventBeginPlay
  (Networking|SwitchHasAuthority
    (:Authority
      (Utilities|Time|SetTimerbyEvent (delegate Custom|SphereTrace) 1.0 true))))

(fn ConstructionScript
  (Components|Box|SetBoxExtent (Variables|Default|GetSpawnerVolume) (Variables|Default|GetBoxExtent) true))