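; Game instance for the MP_FPS game that handles front-end menu navigation and online session management.
; Events create and display the main menu, multiplayer menu and server list widgets, storing a reference to each.
; Single-player and successful non-LAN hosting both open Test_01 by name, without a listen option, and switch to game-only input.
; Separate events join a given search result or destroy the session, with debug prints on host or join failure.
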(event Custom|ShowMultiplayerMenu
  (bind _returnvalue (UserInterface|CreateWidget "/Game/MP_FPS/Widgets/UI/BPW_MultiplayerMenu.BPW_MultiplayerMenu_C" (Game|GetPlayerController 0)))
  (Variables|Default|SetMultiplayerMenuRef _returnvalue)
  (UserInterface|Viewport|AddtoViewport (Variables|Default|GetMultiplayerMenuRef) 0))

(event Custom|ShowMainMenu
  (bind _returnvalue (Game|GetPlayerController 0))
  (bind _returnvalue_2 (UserInterface|CreateWidget "/Game/MP_FPS/Widgets/UI/BPW_MainMenu.BPW_MainMenu_C" _returnvalue))
  (Variables|Default|SetMainMenuRef _returnvalue_2)
  (UserInterface|Viewport|AddtoViewport (Variables|Default|GetMainMenuRef) 0)
  (Input|SetInputModeUIOnly _returnvalue (Variables|Default|GetMainMenuRef) "DoNotLock")
  (Variables|/Script/Engine.PlayerController|SetbShowMouseCursor _returnvalue true))

(event Custom|ShowServerList
  (bind _returnvalue (UserInterface|CreateWidget "/Game/MP_FPS/Widgets/UI/BPW_ServerList.BPW_ServerList_C" (Game|GetPlayerController 0)))
  (Variables|Default|SetServerList _returnvalue)
  (UserInterface|Viewport|AddtoViewport (Variables|Default|GetServerList) 0))

(event Custom|DestroySessionCaller
  (params (PlayerController :type Player%20Controller%20Object%20Reference))
  (|DestroySession PlayerController))

(event Custom|StartSinglePlayer
  (bind _returnvalue (Game|GetPlayerController 0))
  (Game|OpenLevel(byName) "Test_01")
  (Input|SetInputModeGameOnly _returnvalue)
  (Variables|/Script/Engine.PlayerController|SetbShowMouseCursor _returnvalue false))

(event Custom|HostGame
  (bind _returnvalue (Game|GetPlayerController 0))
  (|Session _returnvalue 10 false
    (:OnSuccess
      (Game|OpenLevel(byName) "Test_01" true "listen")
      (Input|SetInputModeGameOnly _returnvalue)
      (Variables|/Script/Engine.PlayerController|SetbShowMouseCursor _returnvalue false))
    (:OnFailure
      (Development|PrintString "Host Game Failed"))))

(event Custom|JoinSession
  (params (Session :type Blueprint%20Session%20Result%20Structure))
  (|JoinSession (Game|GetPlayerController 0) Session
    (:OnFailure
      (Development|PrintString "Failed to join session"))))