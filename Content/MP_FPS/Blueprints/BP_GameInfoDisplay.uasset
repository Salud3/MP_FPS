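; BP_GameInfoDisplay shows the match's game mode and map name on text render components in the FPS multiplayer game.
; On BeginPlay the authority caches the GS_MP_FPS game state in GameStateRef, which has an empty OnRep.
; After a fixed delay, every instance fills both texts from that reference.
; Both texts turn red for competitive modes and green for Co Op or Single Player.
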(event EventBeginPlay
  (bind _txt_gamemode (Variables|Default|GetTXT_GameMode))
  (Utilities|FlowControl|Sequence
    (:then_0
      (Networking|SwitchHasAuthority
        (:Authority
          (Utilities|FlowControl|Sequence
            (:then_0
              (bind _asgs_mp_fps (Utilities|Casting|CastToGS_MP_FPS (Game|GetGameState)))
              (Variables|Default|SetGameStateRef _asgs_mp_fps))))))
    (:then_1
      (Utilities|FlowControl|Delay 5.0)
      (Rendering|Components|TextRender|SetText _txt_gamemode (Utilities|Text|ToText(String) (Utilities|String|EnumtoString (Variables|/Game/MP_FPS/Blueprints/GS_MP_FPS.GS_MP_FPS_C|GetE_SelectedGameMode (Variables|Default|GetGameStateRef)))))
      (Rendering|Components|TextRender|SetText (Variables|Default|GetTXT_MapName) (Utilities|Text|ToText(Name) (Variables|/Game/MP_FPS/Blueprints/GS_MP_FPS.GS_MP_FPS_C|GetSelectedMapName (Variables|Default|GetGameStateRef))))
      (switch Utilities|FlowControl|Switch|SwitchonE_GameModes (Variables|/Game/MP_FPS/Blueprints/GS_MP_FPS.GS_MP_FPS_C|GetE_SelectedGameMode (Variables|Default|GetGameStateRef))
        (:NewEnumerator1
          (Rendering|Components|TextRender|SetTextRenderColor _txt_gamemode (Math|Conversions|ToColor(LinearColor) "(R=1.000000,G=0.000000,B=0.000000,A=1.000000)") :!label _label))
        (:NewEnumerator2
          (goto _label))
        (:NewEnumerator3
          (goto _label))
        (:NewEnumerator4
          (Rendering|Components|TextRender|SetTextRenderColor _txt_gamemode (Math|Conversions|ToColor(LinearColor) "(R=0.000000,G=1.000000,B=0.000000,A=1.000000)") :!label _label_2))
        (:NewEnumerator0
          (goto _label_2))))))

(fn ConstructionScript)

(fn OnRepGameStateRef)