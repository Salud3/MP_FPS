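; Master Blueprint for a team-owned character station in the multiplayer FPS, where players open the character station menu.
; Its trigger volume enables input and sets IsAtStation on the player controller for same-team characters, reversing both on exit.
; Pressing Interact shows the menu through HUD_MP_FPS if the cached character is alive and stationary.
; The construction script colors base and wall meshes by team using dynamic material instances.
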(event OnComponentBeginOverlap(TriggerVolume)
  (params (OverlappedComponent :type Primitive%20Component%20Object%20Reference) (OtherActor :type Actor%20Object%20Reference) (OtherComp :type Primitive%20Component%20Object%20Reference) (OtherBodyIndex :type Integer) (bFromSweep :type Boolean) (SweepResult :type Hit%20Result%20Structure%20%28by%20ref%29))
  (bind _asbp_character_master (Utilities|Casting|CastToBP_Character_Master OtherActor))
  (if (Utilities|Enum|Equal(Enum) (Variables|/Game/MP_FPS/Characters/Blueprints/BP_Character_Master.BP_Character_Master_C|GetTeam _asbp_character_master) (Variables|Default|GetTeam))
    (bind _aspc_mp_fps (Utilities|Casting|CastToPC_MP_FPS (Pawn|GetController _asbp_character_master)))
    (Input|EnableInput _aspc_mp_fps)
    (Variables|/Game/MP_FPS/Blueprints/PC_MP_FPS.PC_MP_FPS_C|SetIsAtStation? _aspc_mp_fps true)))

(event OnComponentEndOverlap(TriggerVolume)
  (params (OverlappedComponent :type Primitive%20Component%20Object%20Reference) (OtherActor :type Actor%20Object%20Reference) (OtherComp :type Primitive%20Component%20Object%20Reference) (OtherBodyIndex :type Integer))
  (bind _asbp_character_master (Utilities|Casting|CastToBP_Character_Master OtherActor))
  (if (Utilities|Enum|Equal(Enum) (Variables|/Game/MP_FPS/Characters/Blueprints/BP_Character_Master.BP_Character_Master_C|GetTeam _asbp_character_master) (Variables|Default|GetTeam))
    (bind _aspc_mp_fps (Utilities|Casting|CastToPC_MP_FPS (Pawn|GetController _asbp_character_master)))
    (Input|DisableInput _aspc_mp_fps)
    (Variables|/Game/MP_FPS/Blueprints/PC_MP_FPS.PC_MP_FPS_C|SetIsAtStation? _aspc_mp_fps false)))

(event Input|ActionEvents|InputActionInteract
  (params (Key :type Key%20Structure :default "AnyKey"))
  (:Pressed
    (Utilities|IsValid (stale OnComponentBeginOverlap(TriggerVolume) _asbp_character_master)
      (:Is%20Valid
        (if (not (Variables|/Game/MP_FPS/Characters/Blueprints/BP_Character_Master.BP_Character_Master_C|GetIsDead? (stale OnComponentBeginOverlap(TriggerVolume) _asbp_character_master)))
          (if (== (Math|Vector|VectorLength (Transformation|GetVelocity (stale OnComponentBeginOverlap(TriggerVolume) _asbp_character_master))) 0.0)
            (bind _ashud_mp_fps (Utilities|Casting|CastToHUD_MP_FPS (HUD|GetHUD (stale OnComponentBeginOverlap(TriggerVolume) _aspc_mp_fps))))
            (Utilities|IsValid _ashud_mp_fps
              (:Is%20Valid
                (Default|ShowCharacterStationMenu _ashud_mp_fps)))))))))

(fn ConstructionScript
  (bind _returnvalue (Rendering|Material|CreateDynamicMaterialInstance (Variables|Default|GetSM_Base) 0 "/Game/MP_FPS/Materials/M_DefaultColor.M_DefaultColor" :!class /Script/Engine.PrimitiveComponent))
  (Variables|Default|SetSM_Base_DynaMat _returnvalue)
  (bind _returnvalue_2 (Rendering|Material|CreateDynamicMaterialInstance (Variables|Default|GetSM_Wall) 0 "/Game/MP_FPS/Materials/M_DefaultColor.M_DefaultColor" :!class /Script/Engine.PrimitiveComponent))
  (Variables|Default|SetSM_Wall_DynaMat _returnvalue_2)
  (Rendering|Material|SetVectorParameterValue (Variables|Default|GetSM_Base_DynaMat) "Color" (Utilities|Select :Index (Variables|Default|GetTeam) :NewEnumerator0 "(R=0.964592,G=0.000000,B=1.000000,A=1.000000)" :NewEnumerator1 "(R=1.000000,G=0.000000,B=0.000000,A=1.000000)" :NewEnumerator2 "(R=0.000000,G=0.000000,B=1.000000,A=1.000000)") :!class /Script/Engine.MaterialInstanceDynamic))