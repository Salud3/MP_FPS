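; Game state for the multiplayer FPS that runs the match countdown, tallies Red and Blue team scores, and stores the game mode and map name.
; BeginPlay reads match length from the game instance, treating 1 as an hour and other values as minutes.
; For all three modes, an authority-only looping timer decrements a timespan each second and formats it as H:M:S text.
; At zero the timer is only cleared; no match-end logic follows.
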(event Custom|Server_SetGSGameInfo
  (params (E_SelectedGameMode :type E_GameModes%20Enum) (SelectedMapName :type Name))
  (Variables|Default|SetE_SelectedGameMode E_SelectedGameMode)
  (Variables|Default|SetSelectedMapName SelectedMapName))

(event Custom|AddScore
  (params (Team :type E_Teams%20Enum) (CoinValue :type Integer))
  (switch Utilities|FlowControl|Switch|SwitchonE_Teams Team
    (:NewEnumerator1
      (Variables|Default|SetRedTeamScore (+ (Variables|Default|GetRedTeamScore) CoinValue)))
    (:NewEnumerator2
      (Variables|Default|SetBlueTeamScore (+ (Variables|Default|GetBlueTeamScore) CoinValue)))))

(event Custom|CountdownTimer
  (bind _timertimespan (Variables|Default|GetTimerTimespan))
  (bind _hours (Variables|Default|GetHours))
  (bind _minutes (Variables|Default|GetMinutes))
  (bind _seconds (Variables|Default|GetSeconds))
  (bind _returnvalue (+ (.seconds _timertimespan) _seconds))
  (bind _returnvalue_2 (+ (.hours _timertimespan) _hours))
  (bind _returnvalue_3 (+ (.minutes _timertimespan) _minutes))
  (bind (_days _hours_2 _minutes_2 _seconds_2) (Math|Timespan|BreakTimespan (Math|Timespan|MakeTimespan (.days _timertimespan) _returnvalue_2 _returnvalue_3 _returnvalue (.milliseconds _timertimespan))))
  (CallFunction|SubtractSeconds)
  (Variables|Default|SetCountdownTimerText (Utilities|Text|FormatText "{H}:{M}:{S}" (Utilities|Text|ToText(Integer) _hours_2 true 1 2) (Utilities|Text|ToText(Integer) _minutes_2 true 2 2) (Utilities|Text|ToText(Integer) _seconds_2 true 2 2)))
  (if (Math|Boolean|ANDBoolean (== _hours_2 0) (== _minutes_2 0) (== _seconds_2 0))
    (Utilities|FlowControl|DoOnce false
      (:Completed
        (Utilities|Time|ClearandInvalidateTimerbyHandle (Variables|Default|GetCountdownTimerHandle))))))

(event EventBeginPlay
  (bind _timertimespan (Variables|Default|GetTimerTimespan))
  (Utilities|FlowControl|Sequence
    (:then_0
      (bind _asgi_mp_fps (Utilities|Casting|CastToGI_MP_FPS (Game|GetGameInstance)))
      (Variables|Default|SetGameInstanceRef _asgi_mp_fps))
    (:then_1
      (if (== (Variables|/Game/MP_FPS/Blueprints/GI_MP_FPS.GI_MP_FPS_C|GetSelectedMatchTime (Variables|Default|GetGameInstanceRef)) 1)
        (Variables|Default|SetHours 1)
        (else
          (Variables|Default|SetMinutes (Variables|/Game/MP_FPS/Blueprints/GI_MP_FPS.GI_MP_FPS_C|GetSelectedMatchTime (Variables|Default|GetGameInstanceRef))))))
    (:then_2
      (switch Utilities|FlowControl|Switch|SwitchonE_GameModes (Variables|/Game/MP_FPS/Blueprints/GI_MP_FPS.GI_MP_FPS_C|GetE_SelectedGameMode (Variables|Default|GetGameInstanceRef))
        (:NewEnumerator1
          _)
        (:NewEnumerator2
          _)
        (:NewEnumerator3
          _))
      (Networking|SwitchHasAuthority
        (:Authority
          (Variables|Default|SetCountdownTimerText (Utilities|Text|FormatText "{H}:{M}:{S}" (Utilities|Text|ToText(Integer) (.Hours (Math|Timespan|BreakTimespan (Math|Timespan|MakeTimespan (.days _timertimespan) (+ (.hours _timertimespan) (Variables|Default|GetHours)) (+ (.minutes _timertimespan) (Variables|Default|GetMinutes)) (+ (.seconds _timertimespan) (Variables|Default|GetSeconds)) (.milliseconds _timertimespan)))) true 1 2) (Utilities|Text|ToText(Integer) (.Minutes (Math|Timespan|BreakTimespan (Math|Timespan|MakeTimespan (.days _timertimespan) (+ (.hours _timertimespan) (Variables|Default|GetHours)) (+ (.minutes _timertimespan) (Variables|Default|GetMinutes)) (+ (.seconds _timertimespan) (Variables|Default|GetSeconds)) (.milliseconds _timertimespan)))) true 2 2) (Utilities|Text|ToText(Integer) (.Seconds (Math|Timespan|BreakTimespan (Math|Timespan|MakeTimespan (.days _timertimespan) (+ (.hours _timertimespan) (Variables|Default|GetHours)) (+ (.minutes _timertimespan) (Variables|Default|GetMinutes)) (+ (.seconds _timertimespan) (Variables|Default|GetSeconds)) (.milliseconds _timertimespan)))) true 2 2)))
          (bind _returnvalue (Utilities|Time|SetTimerbyEvent (delegate Custom|CountdownTimer) 1.0 true))
          (Variables|Default|SetCountdownTimerHandle _returnvalue))))))

(fn ConstructionScript)

(fn SubtractSeconds
  (bind _secondstimespan (Variables|Default|GetSecondsTimespan))
  (Variables|Default|SetTimerTimespan (- (Variables|Default|GetTimerTimespan) (Math|Timespan|MakeTimespan (.days _secondstimespan) (.hours _secondstimespan) (.minutes _secondstimespan) (+ (.seconds _secondstimespan) 1) (.milliseconds _secondstimespan)))))