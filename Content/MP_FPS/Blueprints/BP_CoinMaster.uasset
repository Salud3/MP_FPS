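; BP_CoinMaster is a replicated coin pickup for the multiplayer FPS that adds its value to the collecting character's team score.
; The selected coin type drives both the color of a dynamic material on the cylinder mesh and the score value, set in the construction script and again in its OnRep.
; On overlap with a BP_Character_Master, the authority calls a server event that adds the score through the cached game state and destroys the coin.
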(event Custom|Server_OnActorBeginOverlap
  (params (Character :type BP%20Character%20Master%20Object%20Reference))
  (Default|AddScore (Variables|Default|GetGameStateRef) (Variables|/Game/MP_FPS/Characters/Blueprints/BP_Character_Master.BP_Character_Master_C|GetTeam Character) (Variables|Default|GetCoinValue))
  (Actor|DestroyActor))

(event Collision|EventActorBeginOverlap
  (params (OtherActor :type Actor%20Object%20Reference))
  (Networking|SwitchHasAuthority
    (:Authority
      (bind _asbp_character_master (Utilities|Casting|CastToBP_Character_Master OtherActor))
      (CallFunction|ServeronActorBeginOverlap _asbp_character_master))))

(event EventBeginPlay
  (Networking|SwitchHasAuthority
    (:Authority
      (bind _asgs_mp_fps (Utilities|Casting|CastToGS_MP_FPS (Game|GetGameState)))
      (Variables|Default|SetGameStateRef _asgs_mp_fps))))

(fn ConstructionScript
  (bind _e_selectedcoin (Variables|Default|GetE_SelectedCoin))
  (bind _returnvalue (Rendering|Material|CreateDynamicMaterialInstance (Variables|Default|GetSM_Cylinder) 0 "/Game/MP_FPS/Materials/M_DefaultColor.M_DefaultColor" :!class /Script/Engine.PrimitiveComponent))
  (Variables|Default|SetDynaMatCylinder _returnvalue)
  (Rendering|Material|SetVectorParameterValue (Variables|Default|GetDynaMatCylinder) "Color" (Utilities|Select :Index _e_selectedcoin :NewEnumerator0 "(R=1.000000,G=1.000000,B=1.000000,A=1.000000)" :NewEnumerator1 "(R=0.000000,G=1.000000,B=0.000000,A=1.000000)" :NewEnumerator3 "(R=0.000000,G=0.000000,B=1.000000,A=1.000000)" :NewEnumerator2 "(R=0.088635,G=0.002700,B=0.135000,A=1.000000)" :NewEnumerator4 "(R=0.990000,G=0.096848,B=0.000000,A=1.000000)") :!class /Script/Engine.MaterialInstanceDynamic)
  (Variables|Default|SetCoinValue (Utilities|Select :Index _e_selectedcoin :NewEnumerator0 1 :NewEnumerator1 5 :NewEnumerator3 10 :NewEnumerator2 25 :NewEnumerator4 100)))

(fn OnRepESelectedCoin
  (bind _e_selectedcoin (Variables|Default|GetE_SelectedCoin))
  (Rendering|Material|SetVectorParameterValue (Variables|Default|GetDynaMatCylinder) "Color" (Utilities|Select :Index _e_selectedcoin :NewEnumerator0 "(R=1.000000,G=1.000000,B=1.000000,A=1.000000)" :NewEnumerator1 "(R=0.000000,G=1.000000,B=0.000000,A=1.000000)" :NewEnumerator3 "(R=0.000000,G=0.000000,B=1.000000,A=1.000000)" :NewEnumerator2 "(R=0.088635,G=0.002700,B=0.135000,A=1.000000)" :NewEnumerator4 "(R=0.990000,G=0.096848,B=0.000000,A=1.000000)") :!class /Script/Engine.MaterialInstanceDynamic)
  (Variables|Default|SetCoinValue (Utilities|Select :Index _e_selectedcoin :NewEnumerator0 1 :NewEnumerator1 5 :NewEnumerator3 10 :NewEnumerator2 25 :NewEnumerator4 100)))