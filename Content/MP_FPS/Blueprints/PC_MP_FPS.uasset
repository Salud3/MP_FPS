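; Player controller for the multiplayer FPS that stores the player's team and class and handles respawn requests, the in-game menu and leaving a session.
; Server events set team and class, and respawn requests pass both, plus station status, to GM_MP_FPS.
; Tab opens the menu through GI_MP_FPS.
; EndPlay either has the game instance destroy the session or triggers a client leave that returns to MainMenu.
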(event Custom|Server_RequestRespawn
  (bind _returnvalue (Game|GetGameMode))
  (Utilities|IsValid _returnvalue
    (:Is%20Valid
      (bind _asgm_mp_fps (Utilities|Casting|CastToGM_MP_FPS _returnvalue))
      (Utilities|IsValid _asgm_mp_fps
        (:Is%20Valid
          (Default|ServerRespawnPlayer _asgm_mp_fps self (Variables|Default|GetTeam) (Variables|Default|GetEClass) (Variables|Default|GetIsAtStation?)))))))

(event Custom|Client_LeaveGame
  (|DestroySession self
    (:OnSuccess
      _)
    (:OnFailure
      _))
  (Game|OpenLevel(byName) "MainMenu"))

(event Custom|Server_SetPCTeam
  (params (Team :type E_Teams%20Enum))
  (Variables|Default|SetTeam Team))

(event Custom|Server_SetPCClass
  (params (Class :type E_Classes%20Enum))
  (Variables|Default|SetEClass Class))

(event EventEndPlay
  (params (EndPlayReason :type EEndPlayReason%20Enum :default "Destroyed"))
  (switch Utilities|FlowControl|Switch|SwitchonEEndPlayReason EndPlayReason
    (:Destroyed
      (bind _asgi_mp_fps (Utilities|Casting|CastToGI_MP_FPS (Game|GetGameInstance)))
      (Default|DestroySessionCaller _asgi_mp_fps self))
    (:RemovedFromWorld
      (CallFunction|ClientLeaveGame :!label _label))
    (:Quit
      (goto _label))))

(event EventBeginPlay
  (bind _asgi_mp_fps (Utilities|Casting|CastToGI_MP_FPS (Game|GetGameInstance)))
  (Variables|Default|SetGameInstanceRef _asgi_mp_fps))

(event Input|KeyboardEvents|Tab
  (params (Key :type Key%20Structure :default "AnyKey"))
  (:Pressed
    (Default|ShowinGameMenu (Variables|Default|GetGameInstanceRef) self)))

(fn ConstructionScript)