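; BP_Collectable is a pickup actor that grants a power-up to player characters in the MP_FPS game.
; On actor overlap it casts the other actor to BP_Character_Master and calls PickPowerUp on it.
; It then hides its mesh and disables collision, restoring visibility and query-only collision after a three-second delay so the pickup respawns.
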(event OnComponentBeginOverlap(StaticMesh)
  (params (OverlappedComponent :type Primitive%20Component%20Object%20Reference) (OtherActor :type Actor%20Object%20Reference) (OtherComp :type Primitive%20Component%20Object%20Reference) (OtherBodyIndex :type Integer) (bFromSweep :type Boolean) (SweepResult :type Hit%20Result%20Structure%20%28by%20ref%29)))

(event Custom|DisableCollectable
  (Rendering|SetVisibility (Variables|Default|GetStaticMesh) false false)
  (Collision|SetCollisionEnabled (Variables|Default|GetStaticMesh) "NoCollision")
  (Utilities|FlowControl|Delay 3.0)
  (Rendering|SetVisibility (Variables|Default|GetStaticMesh) true false)
  (Collision|SetCollisionEnabled (Variables|Default|GetStaticMesh) "QueryOnly"))

(event Collision|EventActorBeginOverlap
  (params (OtherActor :type Actor%20Object%20Reference))
  (bind _asbp_character_master (Utilities|Casting|CastToBP_Character_Master OtherActor))
  (bind _output_get (Variables|Default|SetCharacterMasterRef _asbp_character_master))
  (Default|PickPowerUp _output_get)
  (CallFunction|DisableCollectable))

(fn ConstructionScript)