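; Multiplayer FPS game mode that stores the selected mode and map and handles team- and class-based player spawning.
; On authority at BeginPlay, it caches the game instance, then after a short delay sorts team start actors into lobby, red and blue arrays.
; Respawn requests spawn the selected class pawn at a random team start, or at the current pawn's transform when at a station, then possess it.
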(event Custom|Server_SetGMGameInfo
  (params (E_SelectedGameMode :type E_GameModes%20Enum) (SelectedMapName :type Name))
  (Variables|Default|SetE_SelectedGameMode E_SelectedGameMode)
  (Variables|Default|SetSelectedMapName SelectedMapName))

(event Custom|Server_RespawnPlayer
  (params (PlayerController :type Player%20Controller%20Object%20Reference) (Team :type E_Teams%20Enum) (EClass :type E_Classes%20Enum) (IsAtStation :type Boolean))
  (bind _returnvalue (Pawn|GetControlledPawn PlayerController))
  (bind _returnvalue_2 (Utilities|Select :Index EClass :NewEnumerator0 "/Game/MP_FPS/Characters/Blueprints/BPC_Assault.BPC_Assault_C" :NewEnumerator1 "/Game/MP_FPS/Characters/Blueprints/BPC_Biotech.BPC_Biotech_C" :NewEnumerator2 "/Game/MP_FPS/Characters/Blueprints/BPC_Dreadnaught.BPC_Dreadnaught_C" :NewEnumerator3 "/Game/MP_FPS/Characters/Blueprints/BPC_Engineer.BPC_Engineer_C" :NewEnumerator4 "/Game/MP_FPS/Characters/Blueprints/BPC_Recon.BPC_Recon_C"))
  (bind _lobbyspawnpoints (Variables|Default|GetLobbySpawnPoints))
  (bind _redteamspawnpoints (Variables|Default|GetRedTeamSpawnPoints))
  (bind _blueteamspawnpoints (Variables|Default|GetBlueTeamSpawnPoints))
  (bind _returnvalue_3 (Transformation|GetActorTransform _returnvalue))
  (bind _returnvalue_4 (Utilities|Select :Index Team :NewEnumerator0 _lobbyspawnpoints :NewEnumerator1 _redteamspawnpoints :NewEnumerator2 _blueteamspawnpoints))
  (bind _returnvalue_5 (Utilities|Array|Length _returnvalue_4))
  (bind _returnvalue_6 (- _returnvalue_5 1))
  (bind _returnvalue_7 (Math|Random|RandomIntegerinRange 0 _returnvalue_6))
  (bind _item (Utilities|Array|Get(acopy) _returnvalue_4 _returnvalue_7))
  (bind _returnvalue_8 (Transformation|GetActorTransform _item))
  (Utilities|IsValid PlayerController
    (:Is%20Valid
      (if (not IsAtStation)
        (bind _returnvalue_9 (Game|SpawnActorfromClass _returnvalue_2 (Math|Transform|MakeTransform (.location _returnvalue_8) (.rotation _returnvalue_8) "1,1,1") "AdjustIfPossibleButAlwaysSpawn" 0 Team EClass))
        (Utilities|IsValid _returnvalue_9
          (:Is%20Valid
            (Pawn|Possess PlayerController _returnvalue_9)))
        (else
          (bind _returnvalue_10 (Game|SpawnActorfromClass _returnvalue_2 (Math|Transform|MakeTransform (.location _returnvalue_3) (.rotation _returnvalue_3) "1.000000,1,1") "AlwaysSpawn" 0 Team EClass))
          (Utilities|IsValid _returnvalue_10
            (:Is%20Valid
              (Pawn|Possess PlayerController _returnvalue_10))))))))

(event EventBeginPlay
  (Networking|SwitchHasAuthority
    (:Authority
      (Utilities|FlowControl|Sequence
        (:then_0
          (bind _asgi_mp_fps (Utilities|Casting|CastToGI_MP_FPS (Game|GetGameInstance)))
          (Variables|Default|SetGameInstanceRef _asgi_mp_fps))
        (:then_1
          (Utilities|FlowControl|Delay 0.5)
          (bind _outactors (Actor|GetAllActorsOfClass "/Game/MP_FPS/Blueprints/BP_TeamStart_Master.BP_TeamStart_Master_C"))
          (for _array_element _outactors
            (if (Utilities|Enum|Equal(Enum) (Variables|/Game/MP_FPS/Blueprints/BP_TeamStart_Master.BP_TeamStart_Master_C|GetTeam _array_element) "NewEnumerator0")
              (Utilities|Array|Add (Variables|Default|GetLobbySpawnPoints) _array_element)
              (elif (Utilities|Enum|Equal(Enum) (Variables|/Game/MP_FPS/Blueprints/BP_TeamStart_Master.BP_TeamStart_Master_C|GetTeam _array_element) "NewEnumerator1")
                (Utilities|Array|Add (Variables|Default|GetRedTeamSpawnPoints) _array_element)
                (elif (Utilities|Enum|Equal(Enum) (Variables|/Game/MP_FPS/Blueprints/BP_TeamStart_Master.BP_TeamStart_Master_C|GetTeam _array_element) "NewEnumerator2")
                  (Utilities|Array|Add (Variables|Default|GetBlueTeamSpawnPoints) _array_element))))))))))

(fn ConstructionScript)