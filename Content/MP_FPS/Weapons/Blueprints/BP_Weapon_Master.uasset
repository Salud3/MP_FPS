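; Base multiplayer FPS weapon with single, auto and multi-fire modes, hitscan or projectile shots, and scope zoom.
; The client sphere-traces from camera with spread, re-traces from muzzle toward that point, then sends the result to the server.
; The server applies damage or spawns separate first- and third-person projectiles, then multicasts mode-specific effects.
; DoOnce macros limit repeated sounds and owner-filtered muzzle flashes; a timeline drives FOV and HUD scope opacity.
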(event Custom|Client_OnWeaponFire
  (bind _bpcharactermasterref (Variables|Default|GetBPCharacterMasterRef))
  (bind _muzzlesocketname (Variables|Default|GetMuzzleSocketName))
  (bind _array (Utilities|Array|MakeArray _bpcharactermasterref))
  (bind _fp_cam (Variables|/Game/MP_FPS/Characters/Blueprints/BP_Character_Master.BP_Character_Master_C|GetFP_Cam _bpcharactermasterref))
  (bind _returnvalue (Transformation|GetWorldLocation _fp_cam))
  (switch Utilities|FlowControl|Switch|SwitchonE_FiringModes (Variables|Default|GetFiringMode)
    (:NewEnumerator0
      _)
    (:NewEnumerator1
      (Utilities|AutoFireMode
        (:Out
          _)))
    (:NewEnumerator2
      (Utilities|MultiFireMode
        (:Out
          _))))
  (bind (_outhit _returnvalue_2) (Collision|SphereTraceByChannel _returnvalue (Utilities|AddRandomSpread (+ _returnvalue (* (Math|Vector|GetForwardVector (Transformation|GetWorldRotation _fp_cam)) (Variables|Default|GetSphereTraceRange)))) (Variables|Default|GetSphereTraceRadius) "TraceTypeQuery1" false _array "None"))
  (bind (_outhit_2 _returnvalue_3) (Collision|SphereTraceByChannel (Transformation|GetSocketLocation (Variables|Default|GetSK_FP_Weapon) (Variables|Default|GetMuzzleSocketName)) (Math|Vector|SelectVector (.ImpactPoint (Collision|BreakHitResult _outhit)) (.TraceEnd (Collision|BreakHitResult _outhit)) _returnvalue_2) (Variables|Default|GetSphereTraceRadius) "TraceTypeQuery1" false _array "None"))
  (CallFunction|ServerShootInfo _outhit_2 _returnvalue_3 (Transformation|GetSocketLocation (Variables|Default|GetSK_FP_Weapon) _muzzlesocketname) (Transformation|GetSocketLocation (Variables|Default|GetSK_TP_Weapon) _muzzlesocketname)))

(event Custom|Server_ShootInfo
  (params (HitResult :type Hit%20Result%20Structure) (Hit :type Boolean) (FPProjectileSpawnLoc :type Vector) (TPProjectileSpawnLoc :type Vector))
  (bind (_bblockinghit _binitialoverlap _time _location _impactpoint _normal _impactnormal _physmat _hitactor _hitcomponent _hitbonename _hititem _faceindex _tracestart _traceend) (Collision|BreakHitResult HitResult))
  (bind (_bblockinghit_2 _binitialoverlap_2 _time_2 _location_2 _impactpoint_2 _normal_2 _impactnormal_2 _physmat_2 _hitactor_2 _hitcomponent_2 _hitbonename_2 _hititem_2 _faceindex_2 _tracestart_2 _traceend_2) (Collision|BreakHitResult HitResult))
  (if (Variables|Default|GetIsHitscan?)
    (Game|Damage|ApplyDamage (.HitActor (Collision|BreakHitResult HitResult)) (Math|Conversions|ToFloat(Integer) (Variables|Default|GetDamage)) (Game|GetInstigatorController) self)
    (else
      (Game|SpawnActorfromClass (Variables|Default|GetFPProjectile) (Math|Transform|MakeTransform FPProjectileSpawnLoc (Math|Rotator|FindLookatRotation FPProjectileSpawnLoc (Math|Vector|SelectVector _impactpoint _traceend Hit)) "1.000000,1,1") "AlwaysSpawn" (Components|GetOwner) (Game|GetInstigator))
      (Game|SpawnActorfromClass (Variables|Default|GetTPProjectile) (Math|Transform|MakeTransform TPProjectileSpawnLoc (Math|Rotator|FindLookatRotation TPProjectileSpawnLoc (Math|Vector|SelectVector _impactpoint_2 _traceend_2 Hit))) "AlwaysSpawn" (Components|GetOwner) (Game|GetInstigator))))
  (switch Utilities|FlowControl|Switch|SwitchonE_FiringModes (Variables|Default|GetFiringMode)
    (:NewEnumerator0
      (CallFunction|MulticastSingleFireWeaponFX HitResult Hit))
    (:NewEnumerator1
      (CallFunction|MulticastAutoFireFX HitResult Hit))
    (:NewEnumerator2
      (CallFunction|MulticastMultiFireWeaponFx HitResult Hit))))

(event Custom|Multicast_SingleFireWeaponFX
  (params (HitResult :type Hit%20Result%20Structure) (Hit :type Boolean))
  ;[1 1 1] sound and fx
  (CallFunction|SingleFireFX HitResult Hit))

(event Custom|Client_ActivateScope
  (bind _bpcharactermasterref (Variables|Default|GetBPCharacterMasterRef))
  ;[1 1 1] activate/deactivate scope
  (bind (_direction _zoomamount _scopeopacity) (Timeline|ScopeTimeline Play)
    (:Update
      (Camera|SetFieldOfView (Variables|/Game/MP_FPS/Characters/Blueprints/BP_Character_Master.BP_Character_Master_C|GetFP_Cam _bpcharactermasterref) _zoomamount)
      (bind _aspc_mp_fps (Utilities|Casting|CastToPC_MP_FPS (Pawn|GetController _bpcharactermasterref)))
      (bind _ashud_mp_fps (Utilities|Casting|CastToHUD_MP_FPS (HUD|GetHUD _aspc_mp_fps)))
      (Variables|/Game/MP_FPS/Blueprints/HUD_MP_FPS.HUD_MP_FPS_C|SetScopeOpacity _ashud_mp_fps _scopeopacity))))

(event Custom|Client_DeactivateScope
  (bind _bpcharactermasterref (Variables|Default|GetBPCharacterMasterRef))
  ;[1 1 1] activate/deactivate scope
  (bind (_direction _zoomamount _scopeopacity) (Timeline|ScopeTimeline Reverse)
    (:Update
      (Camera|SetFieldOfView (Variables|/Game/MP_FPS/Characters/Blueprints/BP_Character_Master.BP_Character_Master_C|GetFP_Cam _bpcharactermasterref) _zoomamount)
      (bind _aspc_mp_fps (Utilities|Casting|CastToPC_MP_FPS (Pawn|GetController _bpcharactermasterref)))
      (bind _ashud_mp_fps (Utilities|Casting|CastToHUD_MP_FPS (HUD|GetHUD _aspc_mp_fps)))
      (Variables|/Game/MP_FPS/Blueprints/HUD_MP_FPS.HUD_MP_FPS_C|SetScopeOpacity _ashud_mp_fps _scopeopacity))))

(event Custom|Server_OffWeaponFire
  (Utilities|FlowControl|Sequence
    (:then_0
      (Utilities|FlowControl|Delay (Variables|Default|GetWeaponCooldown))
      (Variables|Default|SetIsCooldownActive? false))
    (:then_1
      (CallFunction|MulticastOffWeaponFire))))

(event Custom|Multicast_OffWeaponFire
  ;[1 1 1] sound and fx
  (Utilities|FlowControl|Sequence
    (:then_0
      (Utilities|MultiFireDoOnceFX) ; enters at ResetDoOnce
    )
    (:then_1
      (Utilities|AutoFireSpawnFX) ; enters at ResetDoOnce
    )
    (:then_2
      (Utilities|AutoFireSoundControl) ; enters at ResetDoOnce
    )
    (:then_3
      (Utilities|AutoFireSoundControl) ; enters at FadeOut
    )
    (:then_4
      (Utilities|DestroyAutoFireFX))))

(event Custom|Client_OffWeaponFire
  (bind _bpcharactermasterref (Variables|Default|GetBPCharacterMasterRef))
  (bind _muzzlesocketname (Variables|Default|GetMuzzleSocketName))
  (bind _array (Utilities|Array|MakeArray _bpcharactermasterref))
  (bind _fp_cam (Variables|/Game/MP_FPS/Characters/Blueprints/BP_Character_Master.BP_Character_Master_C|GetFP_Cam _bpcharactermasterref))
  (bind _returnvalue (Transformation|GetWorldLocation _fp_cam))
  (Utilities|FlowControl|Sequence
    (:then_0
      (Utilities|AutoFireMode) ; enters at CloseGate
    )
    (:then_1
      (CallFunction|ServerOffWeaponFire))))

(event Custom|Multicast_AutoFireFX
  (params (HitResult :type Hit%20Result%20Structure) (Hit :type Boolean))
  ;[1 1 1] sound and fx
  (CallFunction|AutoFireFX HitResult Hit)
  (Utilities|FlowControl|Sequence
    (:then_0
      (Utilities|AutoFireSpawnFX))
    (:then_1
      (Utilities|AutoFireSoundControl))))

(event Custom|Multicast_MultiFireWeaponFx
  (params (HitResult :type Hit%20Result%20Structure) (Hit :type Boolean))
  ;[1 1 1] sound and fx
  (Utilities|FlowControl|Sequence
    (:then_0
      (CallFunction|MultiFireFX HitResult Hit))
    (:then_1
      (Utilities|MultiFireDoOnceFX))))

(fn ConstructionScript)

(fn SingleFireFX
  (params (HitResultIn :type Hit%20Result%20Structure%20%28by%20ref%29) (HitIn :type Boolean))
  (bind (_bblockinghit _binitialoverlap _time _location _impactpoint _normal _impactnormal) (Collision|BreakHitResult HitResultIn))
  (bind _sk_fp_weapon (Variables|Default|GetSK_FP_Weapon))
  (bind _muzzlesocketname (Variables|Default|GetMuzzleSocketName))
  (bind _psmuzzleflash (Variables|Default|GetPSMuzzleFlash))
  (Audio|SpawnSoundAttached (Variables|Default|GetSingleFireWeaponSound) _sk_fp_weapon "MuzzleFlash")
  (Utilities|FlowControl|Sequence
    (:then_0
      (bind _returnvalue (Effects|SpawnEmitterAttached _psmuzzleflash _sk_fp_weapon _muzzlesocketname "0, 0, 0" "0, 0, 0" "SnapToTarget"))
      (Rendering|SetOnlyOwnerSee _returnvalue true :!class /Script/Engine.PrimitiveComponent)
      (if (Variables|Default|GetIsHitscan?)
        (if HitIn
          (Audio|PlaySoundatLocation (Variables|Default|GetImpactSound) _impactpoint)
          (Effects|SpawnEmitteratLocation (Variables|Default|GetPSImpact) _impactpoint (Math|Rotator|MakeRotfromZ _impactnormal)))))
    (:then_1
      (bind _returnvalue_2 (Effects|SpawnEmitterAttached _psmuzzleflash (Variables|Default|GetSK_TP_Weapon) _muzzlesocketname "0, 0, 0" "0, 0, 0" "SnapToTarget"))
      (Class|PrimitiveComponent|SetOwnerNoSee _returnvalue_2 true))))

(fn MultiFireFX
  (params (HitResultIn :type Hit%20Result%20Structure%20%28by%20ref%29) (HitIn :type Boolean))
  (bind (_bblockinghit _binitialoverlap _time _location _impactpoint _normal _impactnormal) (Collision|BreakHitResult HitResultIn))
  (if (Variables|Default|GetIsHitscan?)
    (if HitIn
      (Audio|PlaySoundatLocation (Variables|Default|GetImpactSound) _impactpoint)
      (Effects|SpawnEmitteratLocation (Variables|Default|GetPSImpact) _impactpoint (Math|Rotator|MakeRotfromZ _impactnormal)))))

(fn AutoFireFX
  (params (HitResultIn :type Hit%20Result%20Structure%20%28by%20ref%29) (HitIn :type Boolean))
  (bind (_bblockinghit _binitialoverlap _time _location _impactpoint _normal _impactnormal) (Collision|BreakHitResult HitResultIn))
  (if (Variables|Default|GetIsHitscan?)
    (if HitIn
      (Audio|PlaySoundatLocation (Variables|Default|GetImpactSound) _impactpoint)
      (Effects|SpawnEmitteratLocation (Variables|Default|GetPSImpact) _impactpoint (Math|Rotator|MakeRotfromZ _impactnormal)))))

(fn OnRepHasScope?)