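; Master projectile for the multiplayer FPS, handling impacts, effects and damage for bullet and explosive types.
; Bullets act on hit and explosives on projectile stop, with authority-checked server events multicasting hiding, collision shutoff and particles.
; Bullets apply point-of-hit damage on the server, while explosives request radial damage from inside the multicast.
; Third-person copies (IsTPProjectile) skip damage and sound and hide their impact effects from the owner.
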(event OnProjectileStop(ProjectileMovement)
  (params (ImpactResult :type Hit%20Result%20Structure%20%28by%20ref%29))
  (Networking|SwitchHasAuthority
    (:Authority
      (CallFunction|ServeronStop ImpactResult))))

(event Custom|Multicast_OnStop
  (params (HitResult :type Hit%20Result%20Structure))
  (switch Utilities|FlowControl|Switch|SwitchonE_ProjectileTypes (Variables|Default|GetE_ProjectileType)
    (:NewEnumerator1
      (if (not (Variables|Default|GetIsTPProjectile?))
        (Audio|PlaySoundatLocation (Variables|Default|GetExplosionSound) (Transformation|GetActorLocation))
        (CallFunction|ServerApplyDamage HitResult))
      (Development|SetHiddeninGame (Variables|Default|GetSM_Projectile) true false)
      (Collision|SetCollisionEnabled (Variables|Default|GetProjectile_Collision) "NoCollision")
      (bind _returnvalue (Effects|SpawnEmitterAttached (Variables|Default|GetPSExplosion) (Variables|Default|GetProjectile_Collision) "None" "0, 0, 0" "0, 0, 0" "SnapToTarget"))
      (if (Variables|Default|GetIsTPProjectile?)
        (Class|PrimitiveComponent|SetOwnerNoSee _returnvalue true)
        (else
          (Rendering|SetOnlyOwnerSee _returnvalue false :!class /Script/Engine.PrimitiveComponent))))))

(event Custom|ServerApplyDamage
  (params (HitResult :type Hit%20Result%20Structure))
  (if (not (Variables|Default|GetIsTPProjectile?))
    (Game|Damage|ApplyRadialDamage (Math|Conversions|ToFloat(Integer) (Variables|Default|GetDamage)) (Transformation|GetActorLocation) (Variables|Default|GetDamageRadius) 0 0 self (Game|GetInstigatorController) false "ECC_Visibility")))

(event Custom|Server_OnHit
  (params (HitResult :type Hit%20Result%20Structure))
  (if (not (Variables|Default|GetIsTPProjectile?))
    (Game|Damage|ApplyDamage (.HitActor (Collision|BreakHitResult HitResult)) (Math|Conversions|ToFloat(Integer) (Variables|Default|GetDamage)) (Game|GetInstigatorController) self))
  (CallFunction|MulticastonHit HitResult))

(event Custom|Multicast_OnHit
  (params (HitResult :type Hit%20Result%20Structure))
  (if (not (Variables|Default|GetIsTPProjectile?))
    (Audio|PlaySoundatLocation (Variables|Default|GetBulletImpactSound) (.ImpactPoint (Collision|BreakHitResult HitResult))))
  (Development|SetHiddeninGame (Variables|Default|GetSM_Projectile) true false)
  (Collision|SetCollisionEnabled (Variables|Default|GetProjectile_Collision) "NoCollision")
  (bind _returnvalue (Effects|SpawnEmitterAttached (Variables|Default|GetPSBulletImpact) (Variables|Default|GetProjectile_Collision) "None" "0, 0, 0" "0, 0, 0" "SnapToTarget"))
  (if (Variables|Default|GetIsTPProjectile?)
    (Class|PrimitiveComponent|SetOwnerNoSee _returnvalue true)
    (else
      (Rendering|SetOnlyOwnerSee _returnvalue false :!class /Script/Engine.PrimitiveComponent))))

(event Custom|Server_OnStop
  (params (HitResult :type Hit%20Result%20Structure))
  (switch Utilities|FlowControl|Switch|SwitchonE_ProjectileTypes (Variables|Default|GetE_ProjectileType)
    (:NewEnumerator1
      (CallFunction|MulticastonStop HitResult))))

(event Collision|EventHit
  (params (MyComp :type Primitive%20Component%20Object%20Reference) (Other :type Actor%20Object%20Reference) (OtherComp :type Primitive%20Component%20Object%20Reference) (bSelfMoved :type Boolean) (HitLocation :type Vector :default "0, 0, 0") (HitNormal :type Vector :default "0, 0, 0") (NormalImpulse :type Vector :default "0, 0, 0") (Hit :type Hit%20Result%20Structure%20%28by%20ref%29))
  (Networking|SwitchHasAuthority
    (:Authority
      (switch Utilities|FlowControl|Switch|SwitchonE_ProjectileTypes (Variables|Default|GetE_ProjectileType)
        (:NewEnumerator0
          (CallFunction|ServeronHit Hit))))))

(event EventBeginPlay
  (Networking|SwitchHasAuthority
    (:Authority
      (Collision|IgnoreActorwhenMoving (Variables|Default|GetProjectile_Collision) (Game|GetInstigator) true))))

(fn ConstructionScript)